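; Player controller Blueprint that handles basic movement, look and jump input for the player's character.
; Axis events move player pawn 0 forward along the control rotation's yaw and sideways along the controller actor's own right vector.
; Turn and LookUp axes feed controller yaw and pitch, while pressing Jump calls Jump on player character 0.
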(event `InputAxis|FwdMoving`
  (params (AxisValue :type "Float (single-precision)"))
  (bind (_returnvalue_roll _returnvalue_pitch _returnvalue_yaw) (`KismetMathLibrary.BreakRotator` (`self.GetControlRotation`)))
  (`Pawn.AddMovementInput` (`GameplayStatics.GetPlayerPawn` 0) (`KismetMathLibrary.GetForwardVector` (`KismetMathLibrary.MakeRotator` 0.0 0.0 _returnvalue_yaw)) AxisValue false))

(event `InputAxis|RigthMoving`
  (params (AxisValue :type "Float (single-precision)"))
  (`Pawn.AddMovementInput` (`GameplayStatics.GetPlayerPawn` 0) (`self.GetActorRightVector`) AxisValue false))

(event `InputAxis|Turn`
  (params (AxisValue :type "Float (single-precision)"))
  (`self.AddYawInput` AxisValue))

(event `InputAxis|LookUp`
  (params (AxisValue :type "Float (single-precision)"))
  (`self.AddPitchInput` AxisValue))

(event `InputAction|Jump`
  (params (Key :type "Key Structure"))
  (:`Pressed`
    (`Character.Jump` (`GameplayStatics.GetPlayerCharacter` 0))))

(fn `UserConstructionScript`)